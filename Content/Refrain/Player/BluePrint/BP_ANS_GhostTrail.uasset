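; Anim notify state that shows the player's ghost trail effect during a marked window of an animation.
; On begin, it casts the mesh owner to BP_RACharacterPlayer and activates that character's Niagara component without a reset.
; On end, it deactivates the same component, and owners of any other class are ignored.
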(fn ReceivedNotifyBegin
  (params (MeshComp :type Skeletal%20Mesh%20Component%20Object%20Reference) (Animation :type Anim%20Sequence%20Base%20Object%20Reference) (TotalDuration :type Float%20%28single-precision%29) (EventReference :type Anim%20Notify%20Event%20Reference%20Structure%20%28by%20ref%29))
  (bind _asbp_racharacter_player (Utilities|Casting|CastToBP_RACharacterPlayer (Components|GetOwner MeshComp)))
  (Components|Activation|Activate (Variables|/Game/Refrain/Player/BluePrint/BP_RACharacterPlayer.BP_RACharacterPlayer_C|GetNiagara _asbp_racharacter_player) false)
  (return false))

(fn ReceivedNotifyEnd
  (params (MeshComp :type Skeletal%20Mesh%20Component%20Object%20Reference) (Animation :type Anim%20Sequence%20Base%20Object%20Reference) (EventReference :type Anim%20Notify%20Event%20Reference%20Structure%20%28by%20ref%29))
  (bind _asbp_racharacter_player (Utilities|Casting|CastToBP_RACharacterPlayer (Components|GetOwner MeshComp)))
  (Components|Activation|Deactivate (Variables|/Game/Refrain/Player/BluePrint/BP_RACharacterPlayer.BP_RACharacterPlayer_C|GetNiagara _asbp_racharacter_player))
  (return false))